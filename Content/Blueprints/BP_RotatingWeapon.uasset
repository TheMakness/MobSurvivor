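; BP_RotatingWeapon is a timed weapon that orbits the main character and damages enemies it touches.
; On BeginPlay it targets the main character, then destroys itself after BonusTime.
; Each Tick it advances an angle to place itself around the target by rotating a radius vector about Z.
; Enemies overlapping EnemyTrigger take a Health hit every frame, credited to the main character, with no cooldown in this Blueprint.
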(event EventBeginPlay
  (Variables|Default|SetTarget%20Actor (Class|GameUtils|GetMainCharacter))
  (Utilities|FlowControl|Delay (Variables|Default|GetBonusTime))
  (Actor|DestroyActor))

(event EventTick
  (params (DeltaSeconds :type Float%20%28single-precision%29))
  (CallFunction|RotateAroundActor)
  (bind _array_element (Utilities|Array|ForEachLoopwithBreak (Collision|GetOverlappingActors (Variables|Default|GetEnemyTrigger) "/Script/ProgGameplayProto.Enemy" :!class /Script/Engine.PrimitiveComponent))
    (:LoopBody
      (bind _asenemy (Utilities|Casting|CastToEnemy _array_element))
      (Class|Health|HitbyAttack (Variables|/Script/ProgGameplayProto.Enemy|GetHealth _asenemy) (Variables|Default|GetDamageAmount) (Variables|Default|GetTarget%20Actor)))))

(fn ConstructionScript)

(fn RotateAroundActor
  (Variables|Default|SetCurrentAngle (+ (Variables|Default|GetCurrentAngle) (* (Utilities|Time|GetWorldDeltaSeconds) (Variables|Default|GetRotationSpeed))))
  (Transformation|SetActorLocationAndRotation (+ (Transformation|GetActorLocation (Variables|Default|GetTarget%20Actor)) (Math|Vector|RotateVectorAroundAxis (Variables|Default|GetRotationRadius) (Variables|Default|GetCurrentAngle) "0.000000,0.000000,1.000000")) (Math|Rotator|MakeRotator 0.0 (Variables|Default|GetCurrentAngle) 0.0)))