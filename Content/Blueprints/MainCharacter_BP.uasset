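; Player character Blueprint that sets up the game HUD and the level-up flow.
; On BeginPlay it creates the HUD widget, initialized with its Health, Experience and Gold, and pre-creates a level-up widget without displaying it.
; It binds to Experience's level-up event, which pauses the game, shows the stored widget and requests a new set of bonuses.
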(event Custom|OnLevelUp
  (params (NewLevel :type Integer))
  (Game|SetGamePaused true)
  (UserInterface|Viewport|AddtoViewport (Variables|Default|GetLevelUpUI) 0)
  (Default|GetANewSetOfBonuses (Variables|Default|GetLevelUpUI)))

(event EventBeginPlay
  (CallFunction|InitializeHUD)
  (CallFunction|InitializeLevelUp))

(event EventTick
  (params (DeltaSeconds :type Float%20%28single-precision%29)))

(fn ConstructionScript)

(fn InitializeHUD
  (bind _returnvalue (UserInterface|CreateWidget "/Game/UI/GameHUD_UW.GameHUD_UW_C"))
  (UserInterface|Viewport|AddtoViewport _returnvalue 0)
  (Default|Initialize _returnvalue (Variables|Default|GetHealth) (Variables|Default|GetExperience) (Variables|Default|GetGold)))

(fn InitializeLevelUp
  (bind _returnvalue (UserInterface|CreateWidget "/Game/UI/LevelUp_UW.LevelUp_UW_C"))
  (Variables|Default|SetLevelUpUI _returnvalue)
  (EventDispatchers|BindEventtoOnLevelUp (Variables|Default|GetExperience) (EventDispatchers|CreateEvent :!event Custom|OnLevelUp)))