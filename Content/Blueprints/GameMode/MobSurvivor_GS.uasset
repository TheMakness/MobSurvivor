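; MobSurvivor_GS, apparently the game state, initializes permanent upgrades and opens their shop when play begins.
; On BeginPlay it constructs objects from the effect, weapon and power class collections in PermanentUpgrades, storing the instances in three matching collections.
; It then switches the first player to UI-only input, shows the mouse cursor and adds the W_PermanentUpgradeShop widget to the viewport.
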(event EventBeginPlay
  (bind _returnvalue (Game|GetPlayerController 0))
  (bind _permanentupgrades (Variables|Default|GetPermanentUpgrades))
  (bind _result (Utilities|Set|ToArray (.effectpermanentupgrades _permanentupgrades)))
  (for _array_element _result
    (bind _returnvalue_2 (Game|ConstructObjectfromClass _array_element))
    (Utilities|Set|Add (Variables|Default|GetEffectPermanentUpgrades) _returnvalue_2))
  (bind _result_2 (Utilities|Set|ToArray (.weaponpermanentupgrades _permanentupgrades)))
  (for _array_element_2 _result_2
    (bind _returnvalue_3 (Game|ConstructObjectfromClass _array_element_2))
    (Utilities|Set|Add (Variables|Default|GetWeaponPermanentUpgrades) _returnvalue_3))
  (bind _result_3 (Utilities|Set|ToArray (.powerpermanentupgrades _permanentupgrades)))
  (for _array_element_3 _result_3
    (bind _returnvalue_4 (Game|ConstructObjectfromClass _array_element_3))
    (Utilities|Set|Add (Variables|Default|GetPowerPermanentUpgrades) _returnvalue_4))
  (Input|SetInputModeUIOnly _returnvalue 0 "DoNotLock" false)
  (Variables|/Script/Engine.PlayerController|SetbShowMouseCursor (Game|GetPlayerController 0) true)
  (bind _returnvalue_5 (UserInterface|CreateWidget "/Game/UI/PermanentUpgrade/W_PermanentUpgradeShop.W_PermanentUpgradeShop_C" _returnvalue))
  (UserInterface|Viewport|AddtoViewport _returnvalue_5 0))

(fn ConstructionScript)