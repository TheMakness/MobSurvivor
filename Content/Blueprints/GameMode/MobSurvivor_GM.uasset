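; Game mode for MobSurvivor that starts a game with a chosen difficulty preset.
; LoadPreset closes the preset menu, sets GameLevelData to the Easy, Normal or Hard data, with Normal as the fallback, then calls StartGame.
; HidePresetMenu removes the widget and switches to game-only input with the mouse cursor visible.
; The menu creation here is disconnected backup logic, and BeginPlay is empty.
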(event EventBeginPlay)

(fn ConstructionScript)

(fn LoadPreset
  (params (Game%20Preset :type Integer))
  (CallFunction|HidePresetMenu)
  (switch int Game%20Preset
    (:Default
      (Variables|Default|SetGameLevelData (Variables|Default|GetGamePresetNormal) :!label _label))
    (:0
      (Variables|Default|SetGameLevelData (Variables|Default|GetGamePresetEasy)))
    (:1
      (goto _label))
    (:2
      (Variables|Default|SetGameLevelData (Variables|Default|GetGamePresetHard))))
  (Class|ProgGameplayProtoGameMode|StartGame))

(fn HidePresetMenu
  (Input|SetInputModeGameOnly (Game|GetPlayerController 0) false)
  (Variables|/Script/Engine.PlayerController|SetbShowMouseCursor (Game|GetPlayerController 0) true)
  (Widget|RemovefromParent (Variables|Default|GetGame%20Preset%20Menu%20Widget)))