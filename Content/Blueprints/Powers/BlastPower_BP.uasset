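; BlastPower_BP is a power that, on Use, sends out an expanding blast that damages what it touches.
; Unless the countdown has started, it calls the parent Use, then enables a query-only sphere that a timeline grows from zero to Radius.
; Each actor the sphere begins overlapping takes Damage through its Health component, if it has one.
; When the timeline finishes, the sphere's collision is disabled and its radius reset.
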(event OnComponentBeginOverlap(Sphere)
  (params (OverlappedComponent :type Primitive%20Component%20Object%20Reference) (OtherActor :type Actor%20Object%20Reference) (OtherComp :type Primitive%20Component%20Object%20Reference) (OtherBodyIndex :type Integer) (bFromSweep :type Boolean) (SweepResult :type Hit%20Result%20Structure%20%28by%20ref%29))
  (bind _returnvalue (Actor|GetComponentbyClass OtherActor "/Script/ProgGameplayProto.Health"))
  (Utilities|IsValid _returnvalue
    (:Is%20Valid
      (Class|Health|HitbyAttack _returnvalue (Variables|Default|GetDamage)))))

(event EventBeginPlay)

(event Collision|EventActorBeginOverlap
  (params (OtherActor :type Actor%20Object%20Reference)))

(event EventTick
  (params (DeltaSeconds :type Float%20%28single-precision%29)))

(event EventUse
  (if (not (Variables|Default|GetIsCountdownStart))
    (|CallParentFunction)
    (CallFunction|InitCollider)
    (bind _alpha (Timeline|Blast_T PlayFromStart)
      (:Update
        (Components|Sphere|SetSphereRadius (Variables|Default|GetSphere) (Math|Float|Lerp 0.0 (Variables|Default|GetRadius) _alpha) true))
      (:Finished
        (CallFunction|DisableCollider)))))

(fn ConstructionScript)

(fn InitCollider
  (Components|Sphere|SetSphereRadius (Variables|Default|GetSphere) 0.0 false)
  (Collision|SetCollisionEnabled (Variables|Default|GetSphere) "QueryOnly"))

(fn DisableCollider
  (Collision|SetCollisionEnabled (Variables|Default|GetSphere) "NoCollision")
  (Components|Sphere|SetSphereRadius (Variables|Default|GetSphere) 0.0 false))