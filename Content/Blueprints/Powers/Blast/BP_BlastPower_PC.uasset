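; BP_BlastPower_PC is a power component that gives its owning actor a blast ability.
; On BeginPlay it spawns a BP_BlastSphere at the owner's transform, passing the owner as instigator if it is a Pawn, and attaches it to itself.
; UseBehaviour triggers IgniteBlast on that stored sphere, so each use reuses the same actor rather than spawning a new one.
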(event EventBeginPlay
  (bind _returnvalue (Components|GetOwner))
  (bind _returnvalue_2 (Transformation|GetActorTransform _returnvalue))
  (bind _aspawn (Utilities|Casting|CastToPawn (Components|GetOwner))
    (:then
      (bind _returnvalue_3 (Game|SpawnActorfromClass "/Game/Blueprints/Powers/Blast/BP_BlastSphere.BP_BlastSphere_C" _returnvalue_2 "Undefined" "MultiplyWithRoot" 0 _aspawn))
      (Variables|Default|SetBlastActor _returnvalue_3))
    (:CastFailed
      (bind _returnvalue_4 (Game|SpawnActorfromClass "/Game/Blueprints/Powers/Blast/BP_BlastSphere.BP_BlastSphere_C" _returnvalue_2 "Undefined" "MultiplyWithRoot" 0 0))
      (Variables|Default|SetBlastActor _returnvalue_4)))
  (Transformation|AttachComponentToComponent (Variables|Default|GetBlastActor) self "None" "KeepRelative" "KeepRelative" "KeepRelative" true))

(event EventUseBehaviour
  (Default|IgniteBlast (Variables|Default|GetBlastActor)))