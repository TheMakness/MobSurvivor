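; MobSurvivor game mode Blueprint that lets the player pick a difficulty preset before gameplay starts.
; On BeginPlay it shows the preset menu widget with UI-only input and a visible cursor.
; LoadPreset removes the menu, switches to game-only input while keeping the cursor visible, then sets GameLevelData to the Easy, Normal or Hard preset, defaulting to Normal, and calls StartGame.
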(event EventBeginPlay
  (Input|SetInputModeUIOnly (Game|GetPlayerController 0) 0 "DoNotLock" false)
  (Variables|/Script/Engine.PlayerController|SetbShowMouseCursor (Game|GetPlayerController 0) true)
  (bind _returnvalue (UserInterface|CreateWidget "/Game/UI/W_GamePresetMenu.W_GamePresetMenu_C"))
  (bind _output_get (Variables|Default|SetGame%20Preset%20Menu%20Widget _returnvalue))
  (UserInterface|Viewport|AddtoViewport _output_get 0))

(fn ConstructionScript)

(fn LoadPreset
  (params (Game%20Preset :type Integer))
  (CallFunction|HidePresetMenu)
  (switch int Game%20Preset
    (:Default
      (Variables|Default|SetGameLevelData (Variables|Default|GetGamePresetNormal) :!label _label))
    (:0
      (Variables|Default|SetGameLevelData (Variables|Default|GetGamePresetEasy)))
    (:1
      (goto _label))
    (:2
      (Variables|Default|SetGameLevelData (Variables|Default|GetGamePresetHard))))
  (Class|ProgGameplayProtoGameMode|StartGame))

(fn HidePresetMenu
  (Input|SetInputModeGameOnly (Game|GetPlayerController 0) false)
  (Variables|/Script/Engine.PlayerController|SetbShowMouseCursor (Game|GetPlayerController 0) true)
  (Widget|RemovefromParent (Variables|Default|GetGame%20Preset%20Menu%20Widget)))