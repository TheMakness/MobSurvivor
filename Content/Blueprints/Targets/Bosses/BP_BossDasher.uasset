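; BP_BossDasher is a boss target that flashes its mesh when a projectile hits it.
; On BeginPlay it creates a dynamic instance of the mesh's first material and applies it.
; Each hit sets that material's BlinkAlpha parameter to full, waits BlinkTime, then resets it to zero.
; The graph holds only this hit feedback, with no dash, movement or damage logic.
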(event EventOnHitByProjectile
  (params (Projectile :type Weapon%20Projectile%20Object%20Reference))
  (Rendering|Material|SetScalarParameterValue (Variables|Default|GetMaterialInstance) "BlinkAlpha" 1.0 :!class /Script/Engine.MaterialInstanceDynamic)
  (Utilities|FlowControl|Delay (Variables|Default|GetBlinkTime))
  (Rendering|Material|SetScalarParameterValue (Variables|Default|GetMaterialInstance) "BlinkAlpha" 0.0 :!class /Script/Engine.MaterialInstanceDynamic))

(event EventBeginPlay
  (bind _returnvalue (Rendering|Material|CreateDynamicMaterialInstance (Variables|Default|GetStaticMesh) 0 (Rendering|Material|GetMaterial (Variables|Default|GetStaticMesh) 0) "None" :!class /Script/Engine.PrimitiveComponent))
  (bind _output_get (Variables|Default|SetMaterialInstance _returnvalue))
  (Rendering|Material|SetMaterial (Variables|Default|GetStaticMesh) 0 _output_get))

(fn ConstructionScript)